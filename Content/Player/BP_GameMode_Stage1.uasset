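; Game mode for Stage 1 that detects the boss's defeat and presents the stage-clear screen.
; On BeginPlay it caches the BP_Boss tagged "Boss" and adds a hidden WB_StageClear widget to the viewport.
; Tick polls the boss's StateType for what appears to be its death state, then fires once through DoOnce.
; That triggers brief slow motion with a camera shake, then shows the widget and mouse cursor.
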(event `self.ReceiveBeginPlay`
  (bind _outactors (`GameplayStatics.GetAllActorsOfClass` "/Game/Boss/BP_Boss.BP_Boss_C"))
  (for _array_element _outactors
    (for _array_element_2 (`Actor.Tags` _array_element)
      (if (== _array_element_2 "Boss")
        (set `self.Boss` _array_element)
        (bind _returnvalue (`|CreateWidget` "/Game/UI/WB_StageClear.WB_StageClear_C"))
        (bind _output_get (set `self.StageClearWidget` _returnvalue))
        (`UserWidget.AddToViewport` _output_get 0)
        (`Widget.SetVisibility` (`self.StageClearWidget`) "Hidden")))))

(event `self.ReceiveTick`
  (params (DeltaSeconds :type "Float (single-precision)"))
  (bind _boss (`self.Boss`)
    (:`then`
      (if (`|EnumEquality` (`/Game/Boss/BP_Boss.StateType` _boss) "NewEnumerator3")
        (`/Engine/EditorBlueprintResources/StandardMacros.DoOnce` false
          (:`Completed`
            (`|ExecutionSequence`
              (:`then_0`
                (`GameplayStatics.SetGlobalTimeDilation` 0.25)
                (`PlayerCameraManager.PlayCameraShake` :`self` (`GameplayStatics.GetPlayerCameraManager` 0) :`ShakeClass` "/Game/Player/Shake_BossDead.Shake_BossDead_C")
                (`KismetSystemLibrary.Delay` 0.15)
                (`GameplayStatics.SetGlobalTimeDilation` 1.0))
              (:`then_1`
                (`Widget.SetVisibility` (`self.StageClearWidget`) "Visible")
                (set `PlayerController.bShowMouseCursor` true (`GameplayStatics.GetPlayerController` 0))))))))
    (:`else`)))

(fn `UserConstructionScript`)