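; Camera actor that follows the first player character at a fixed offset.
; On BeginPlay it stores its placed offset from the character's location.
; Each Tick it sets its location to the character's position plus that offset, without sweeping, smoothing or changing rotation.
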(event `self.ReceiveBeginPlay`
  (set `self.Offset` (- (`self.K2_GetActorLocation`) (`self.K2_GetActorLocation` (`GameplayStatics.GetPlayerCharacter` 0)))))

(event `self.ReceiveTick`
  (params (DeltaSeconds :type "Float (single-precision)"))
  (`self.K2_SetActorLocation` (+ (`self.Offset`) (`self.K2_GetActorLocation` (`GameplayStatics.GetPlayerCharacter` 0)))))

(fn `UserConstructionScript`)