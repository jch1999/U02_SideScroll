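; Player character Blueprint with sideways movement, jumping and a sword slash attack, viewed through its MainCamera set as view target on BeginPlay.
; An Attacking flag blocks movement, jumping and repeat attacks once a slash montage starts; nothing here clears it.
; OnCollison and OffCollision events toggle the sword's collision, whose overlaps only print the other actor's name.
; Forward movement logic exists but is disconnected, leaving movement on the world Y axis.
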(event `self.ReceiveBeginPlay`
  ;[1 1 1] BeginPlay
  (`PlayerController.SetViewTargetWithBlend` (`GameplayStatics.GetPlayerController` 0) (`self.MainCamera`) 0.0 "VTBlend_Linear" 0.0 false)
  (`PrimitiveComponent.SetCollisionEnabled` (`self.SwordCollision`) "NoCollision"))

(event `Key|SpaceBar`
  (params (Key :type "Key Structure"))
  ;[1 1 1] 점프
  (:`Pressed`
    (if (not (`self.bAttacking`))
      (`self.Jump`)))
  (:`Released`
    (`self.StopJumping`)))

(event `InputAxis|MoveForward`
  (params (AxisValue :type "Float (single-precision)"))
  ;[1 1 1] 이동
)

(event `InputAxis|MoveRight`
  (params (AxisValue :type "Float (single-precision)"))
  ;[1 1 1] 이동
  (if (not (`self.bAttacking`))
    (`self.AddMovementInput` (0.0 1.0 0.0) AxisValue)))

(event `Key|LeftMouseButton`
  (params (Key :type "Key Structure"))
  ;[1 1 1] 공격
  (:`Pressed`
    (if (not (`self.bAttacking`))
      (set `self.bAttacking` true)
      (`self.PlayAnimMontage` "/Game/Mixamo/Paladin/Animations/sword_and_shield_slash_Montage.sword_and_shield_slash_Montage" 1.2))))

(event `self.SwordCollision.OnComponentBeginOverlap`
  (params (OverlappedComponent :type "PrimitiveComponent Object Reference") (OtherActor :type "Actor Object Reference") (OtherComp :type "PrimitiveComponent Object Reference") (OtherBodyIndex :type Integer) (bFromSweep :type Boolean) (SweepResult :type "HitResult Structure (by ref)"))
  (if (!= OtherActor self)
    (`KismetSystemLibrary.PrintString` (`KismetSystemLibrary.GetDisplayName` OtherActor))))

(event `OnCollison`
  ;[1 1 1] SwordCollision On/Off
  (`PrimitiveComponent.SetCollisionEnabled` (`self.SwordCollision`) "QueryAndPhysics"))

(event `OffCollision`
  ;[1 1 1] SwordCollision On/Off
  (`PrimitiveComponent.SetCollisionEnabled` (`self.SwordCollision`) "NoCollision"))

(fn `UserConstructionScript`)