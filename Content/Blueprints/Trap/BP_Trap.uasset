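; Trap actor that spins continuously on Tick and damages Characters standing inside its overlap area.
; Overlap begin and end events add and remove Characters in a tracked list, and each begin sets a fast looping timer for TakeDamage.
; TakeDamage applies Atk damage to every tracked Character unless BP_GameModeBase flags IsEnd.
; The timer is never cleared, so it keeps polling after the list empties.
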(event `self.ReceiveTick`
  (params (DeltaSeconds :type "Float (single-precision)"))
  (`self.K2_AddActorWorldRotation` (struct :`Roll` 10.0)))

(event `self.ReceiveActorBeginOverlap`
  (params (OtherActor :type "Actor Object Reference"))
  (bind _ascharacter (cast `Character` OtherActor))
  (`KismetArrayLibrary.Array_AddUnique` (`self.HittedCharcters`) _ascharacter)
  (`KismetSystemLibrary.K2_SetTimer` self "TakeDamage" 0.1 true))

(event `self.ReceiveActorEndOverlap`
  (params (OtherActor :type "Actor Object Reference"))
  (bind _ascharacter (cast `Character` OtherActor))
  (`KismetArrayLibrary.Array_RemoveItem` (`self.HittedCharcters`) _ascharacter))

(fn `TakeDamage`
  (bind _hittedcharcters (`self.HittedCharcters`))
  (bind _asbp_game_mode_base (cast `/Game/Game/BP_GameModeBase` (`GameplayStatics.GetGameMode`)))
  (if (not (or (`/Game/Game/BP_GameModeBase.IsEnd` _asbp_game_mode_base) (< (`KismetArrayLibrary.Array_Length` _hittedcharcters) 1)))
    (for _array_element _hittedcharcters
      (`GameplayStatics.ApplyDamage` _array_element (`self.Atk`) null self))))

(fn `UserConstructionScript`)