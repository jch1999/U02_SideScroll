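; BP_PressTrap is a press trap that starts moving when a character first enters its detection box and damages characters it hits.
; A timeline lerps the mesh along its up vector by FallDist, replaying endlessly because the detected flag never resets.
; The timeline's vector track drives position with X and toggles the damage box collision with Y.
; Characters take Atk damage on entering that box, tracked to avoid duplicate hits until they leave.
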(event `self.ReceiveBeginPlay`
  (bind _staticmesh (`self.StaticMesh`))
  (bind _output_get (set `self.StartPos` (`SceneComponent.K2_GetComponentLocation` _staticmesh)))
  (set `self.EndPos` (+ _output_get (* (`SceneComponent.GetUpVector` _staticmesh) (`self.FallDist`)))))

(event `self.DetectCollision(Box).OnComponentBeginOverlap`
  (params (OverlappedComponent :type "PrimitiveComponent Object Reference") (OtherActor :type "Actor Object Reference") (OtherComp :type "PrimitiveComponent Object Reference") (OtherBodyIndex :type Integer) (bFromSweep :type Boolean) (SweepResult :type "HitResult Structure (by ref)"))
  (bind _damagecollision_box_ (`self.DamageCollision(Box)`))
  (bind _ascharacter (cast `Character` OtherActor))
  (`KismetArrayLibrary.Array_AddUnique` (`self.DetectedCharacters`) _ascharacter)
  (if (not (`self.bIsDetected`))
    (set `self.bIsDetected` true)
    (if (`self.bIsDetected`) :!label _label
      (`TimelineComponent.SetPlayRate` (`self.PressPosAlpha`) (`self.TileLineSpd`))
      (bind (_direction _alpha_damageable) (`Timeline|PressPosAlpha` :!via `PlayFromStart`)
        (:`Update`
          (`SceneComponent.K2_SetWorldLocation` (`self.StaticMesh`) (`KismetMathLibrary.VLerp` (`self.StartPos`) (`self.EndPos`) (.x _alpha_damageable)) false false)
          (if (>= (.y _alpha_damageable) 1.0)
            (`PrimitiveComponent.SetCollisionEnabled` _damagecollision_box_ "QueryAndPhysics")
            (else
              (`PrimitiveComponent.SetCollisionEnabled` _damagecollision_box_ "NoCollision"))))
        (:`Finished`
          (goto _label))))))

(event `self.DetectCollision(Box).OnComponentEndOverlap`
  (params (OverlappedComponent :type "PrimitiveComponent Object Reference") (OtherActor :type "Actor Object Reference") (OtherComp :type "PrimitiveComponent Object Reference") (OtherBodyIndex :type Integer))
  (bind _ascharacter (cast `Character` OtherActor))
  (`KismetArrayLibrary.Array_RemoveItem` (`self.DetectedCharacters`) _ascharacter))

(event `self.DamageCollision(Box).OnComponentBeginOverlap`
  (params (OverlappedComponent :type "PrimitiveComponent Object Reference") (OtherActor :type "Actor Object Reference") (OtherComp :type "PrimitiveComponent Object Reference") (OtherBodyIndex :type Integer) (bFromSweep :type Boolean) (SweepResult :type "HitResult Structure (by ref)"))
  (bind _hittedcharacters (`self.HittedCharacters`))
  (bind _ascharacter (cast `Character` OtherActor))
  (bind _returnvalue (`KismetArrayLibrary.Array_AddUnique` _hittedcharacters _ascharacter))
  (if (`KismetArrayLibrary.Array_IsValidIndex` _hittedcharacters _returnvalue)
    (`GameplayStatics.ApplyDamage` _ascharacter (`self.Atk`) null self)))

(event `self.DamageCollision(Box).OnComponentEndOverlap`
  (params (OverlappedComponent :type "PrimitiveComponent Object Reference") (OtherActor :type "Actor Object Reference") (OtherComp :type "PrimitiveComponent Object Reference") (OtherBodyIndex :type Integer))
  (bind _ascharacter (cast `Character` OtherActor))
  (`KismetArrayLibrary.Array_RemoveItem` (`self.HittedCharacters`) _ascharacter))

(fn `UserConstructionScript`)