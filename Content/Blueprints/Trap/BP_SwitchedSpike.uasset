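; BP_SwitchedSpike is a spike trap actor that moves along its up axis and damages characters touching it.
; A character entering the trigger box starts a timeline that lerps between start and raised positions, replaying while active.
; Leaving the trigger stops replays only if no characters remain in the damage box.
; Damage-box overlaps maintain a character list and start a looping, never-cleared timer that applies damage to everyone listed.
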(event `self.ReceiveBeginPlay`
  (set `self.Start` (`self.K2_GetActorLocation`))
  (set `self.End` (+ (`self.Start`) (* (`self.GetActorUpVector`) 300.0))))

(event `self.DamageArea(Box).OnComponentBeginOverlap`
  (params (OverlappedComponent :type "PrimitiveComponent Object Reference") (OtherActor :type "Actor Object Reference") (OtherComp :type "PrimitiveComponent Object Reference") (OtherBodyIndex :type Integer) (bFromSweep :type Boolean) (SweepResult :type "HitResult Structure (by ref)"))
  (bind _ascharacter (cast `Character` OtherActor))
  (`KismetArrayLibrary.Array_AddUnique` (`self.HittedCharacters`) _ascharacter)
  (`KismetSystemLibrary.K2_SetTimer` self "TakeDamage" 0.3 true))

(event `self.DamageArea(Box).OnComponentEndOverlap`
  (params (OverlappedComponent :type "PrimitiveComponent Object Reference") (OtherActor :type "Actor Object Reference") (OtherComp :type "PrimitiveComponent Object Reference") (OtherBodyIndex :type Integer))
  (bind _ascharacter (cast `Character` OtherActor))
  (`KismetArrayLibrary.Array_RemoveItem` (`self.HittedCharacters`) _ascharacter))

(event `self.TriggerArea(Box).OnComponentBeginOverlap`
  (params (OverlappedComponent :type "PrimitiveComponent Object Reference") (OtherActor :type "Actor Object Reference") (OtherComp :type "PrimitiveComponent Object Reference") (OtherBodyIndex :type Integer) (bFromSweep :type Boolean) (SweepResult :type "HitResult Structure (by ref)"))
  (cast `Character` OtherActor)
  (`TimelineComponent.SetPlayRate` (`self.TimeLine`) (`self.TimeLineSpd`))
  (set `self.bIsActive` true)
  (if (`self.bIsActive`) :!label _label
    (bind (_direction _alpha) (`Timeline|TimeLine` :!via `PlayFromStart`)
      (:`Update`
        (`self.K2_SetActorLocation` (`KismetMathLibrary.VLerp` (`self.Start`) (`self.End`) _alpha)))
      (:`Finished`
        (goto _label)))))

(event `self.TriggerArea(Box).OnComponentEndOverlap`
  (params (OverlappedComponent :type "PrimitiveComponent Object Reference") (OtherActor :type "Actor Object Reference") (OtherComp :type "PrimitiveComponent Object Reference") (OtherBodyIndex :type Integer))
  (cast `Character` OtherActor)
  (if (== (`KismetArrayLibrary.Array_Length` (`self.HittedCharacters`)) 0)
    (set `self.bIsActive` false)))

(fn `TakeDamage`
  (bind _hittedcharacters (`self.HittedCharacters`))
  (if (not (< (`KismetArrayLibrary.Array_Length` _hittedcharacters) 1))
    (for _array_element _hittedcharacters
      (`GameplayStatics.ApplyDamage` _array_element (`self.Atk`) null self))))

(fn `UserConstructionScript`)