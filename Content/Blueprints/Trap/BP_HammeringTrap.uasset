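; BP_HammeringTrap is a trap that swings a hammer repeatedly while characters stand in its detection area, damaging those it hits.
; A looping timeline drives the mesh rotation from start to target with one curve channel and gates hitbox collision with another.
; DetectAreaBox tracks occupants to keep the loop running, letting the current swing finish once empty.
; The hitbox tracks overlapping characters, applying damage only when one is newly added.
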(event `self.ReceiveBeginPlay`
  (set `self.StartRot` (`SceneComponent.K2_GetComponentRotation` (`self.SkeletalMesh`))))

(event `self.DetectArea(Box).OnComponentBeginOverlap`
  (params (OverlappedComponent :type "PrimitiveComponent Object Reference") (OtherActor :type "Actor Object Reference") (OtherComp :type "PrimitiveComponent Object Reference") (OtherBodyIndex :type Integer) (bFromSweep :type Boolean) (SweepResult :type "HitResult Structure (by ref)"))
  (bind _box (`self.Box`))
  (bind _ascharacter (cast `Character` OtherActor))
  (`KismetArrayLibrary.Array_AddUnique` (`self.DetectedCharacters`) _ascharacter)
  (if (not (`self.bIsDetected`))
    (set `self.bIsDetected` true)
    (if (`self.bIsDetected`) :!label _label
      (`TimelineComponent.SetPlayRate` (`self.HammerRotatingAlpha`) (`self.TimeLinePlayRate`))
      (bind (_direction _alpha_damageable) (`Timeline|HammerRotatingAlpha` :!via `PlayFromStart`)
        (:`Update`
          (`SceneComponent.K2_SetWorldRotation` (`self.SkeletalMesh`) (`KismetMathLibrary.RLerp` (`self.StartRot`) (`self.TargetRot`) (.x _alpha_damageable) true) false false)
          (if (>= (.y _alpha_damageable) 1.0)
            (`PrimitiveComponent.SetCollisionEnabled` _box "QueryAndPhysics")
            (else
              (`PrimitiveComponent.SetCollisionEnabled` _box "NoCollision"))))
        (:`Finished`
          (goto _label))))))

(event `self.DetectArea(Box).OnComponentEndOverlap`
  (params (OverlappedComponent :type "PrimitiveComponent Object Reference") (OtherActor :type "Actor Object Reference") (OtherComp :type "PrimitiveComponent Object Reference") (OtherBodyIndex :type Integer))
  (bind _ascharacter (cast `Character` OtherActor))
  (`KismetArrayLibrary.Array_RemoveItem` (`self.DetectedCharacters`) _ascharacter)
  (if (== (`KismetArrayLibrary.Array_Length` (`self.DetectedCharacters`)) 0)
    (set `self.bIsDetected` false)))

(event `self.Box.OnComponentBeginOverlap`
  (params (OverlappedComponent :type "PrimitiveComponent Object Reference") (OtherActor :type "Actor Object Reference") (OtherComp :type "PrimitiveComponent Object Reference") (OtherBodyIndex :type Integer) (bFromSweep :type Boolean) (SweepResult :type "HitResult Structure (by ref)"))
  (bind _hittedcharacters (`self.HittedCharacters`))
  (bind _ascharacter (cast `Character` OtherActor))
  (bind _returnvalue (`KismetArrayLibrary.Array_AddUnique` _hittedcharacters _ascharacter))
  (if (`KismetArrayLibrary.Array_IsValidIndex` _hittedcharacters _returnvalue)
    (`GameplayStatics.ApplyDamage` _ascharacter (`self.Atk`) null self)))

(event `self.Box.OnComponentEndOverlap`
  (params (OverlappedComponent :type "PrimitiveComponent Object Reference") (OtherActor :type "Actor Object Reference") (OtherComp :type "PrimitiveComponent Object Reference") (OtherBodyIndex :type Integer))
  (bind _ascharacter (cast `Character` OtherActor))
  (`KismetArrayLibrary.Array_RemoveItem` (`self.HittedCharacters`) _ascharacter))

(fn `UserConstructionScript`)