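; BP_AutoSpike is a spike trap that moves on its own and damages characters touching it.
; On BeginPlay a timeline lerps it from its start location along its up vector, with configurable distance and play rate.
; Overlaps maintain a list of characters and start a looping timer that is never cleared.
; Each tick of that timer applies damage and a particle effect to listed characters unless the game mode has ended.
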(event `self.ReceiveBeginPlay`
  (set `self.Start` (`self.K2_GetActorLocation`))
  (set `self.End` (+ (`self.Start`) (* (`self.GetActorUpVector`) (`self.MoveDist`))))
  (`TimelineComponent.SetPlayRate` (`self.TimeLine`) (`self.TimeLineSpd`))
  (bind (_direction _alpha) (`Timeline|TimeLine`)
    (:`Update`
      (`self.K2_SetActorLocation` (`KismetMathLibrary.VLerp` (`self.Start`) (`self.End`) _alpha)))))

(event `self.ReceiveActorBeginOverlap`
  (params (OtherActor :type "Actor Object Reference"))
  (bind _ascharacter (cast `Character` OtherActor))
  (`KismetArrayLibrary.Array_AddUnique` (`self.HittedCharacters`) _ascharacter)
  (`KismetSystemLibrary.K2_SetTimer` self "TakeDamage" 0.3 true))

(event `self.ReceiveActorEndOverlap`
  (params (OtherActor :type "Actor Object Reference"))
  (bind _ascharacter (cast `Character` OtherActor))
  (`KismetArrayLibrary.Array_RemoveItem` (`self.HittedCharacters`) _ascharacter))

(event `self.Spike(StaticMesh).OnComponentBeginOverlap`
  (params (OverlappedComponent :type "PrimitiveComponent Object Reference") (OtherActor :type "Actor Object Reference") (OtherComp :type "PrimitiveComponent Object Reference") (OtherBodyIndex :type Integer) (bFromSweep :type Boolean) (SweepResult :type "HitResult Structure (by ref)")))

(fn `TakeDamage`
  (bind _hittedcharacters (`self.HittedCharacters`))
  (bind _asbp_game_mode_base (cast `/Game/Game/BP_GameModeBase` (`GameplayStatics.GetGameMode`)))
  (if (not (or (`/Game/Game/BP_GameModeBase.IsEnd` _asbp_game_mode_base) (< (`KismetArrayLibrary.Array_Length` _hittedcharacters) 1)))
    (for _array_element _hittedcharacters
      (`GameplayStatics.ApplyDamage` _array_element (`self.Atk`) null self)
      (`GameplayStatics.SpawnEmitterAtLocation` "/Game/InfinityBladeEffects/Effects/FX_Ability/Heal/P_Heal_Pickup.P_Heal_Pickup" (`self.K2_GetActorLocation` _array_element)))))

(fn `UserConstructionScript`)