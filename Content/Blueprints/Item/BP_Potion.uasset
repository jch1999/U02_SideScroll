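; BP_Potion is a health potion item that bobs along its up axis and can restore HP to a player.
; On BeginPlay, the RoundTrip timeline drives a location lerp between the start point and a short offset above it.
; IncreaseHP adds Amount to the given player's HP, clamped to MaxHP.
; The mesh overlap event is empty, and nothing in this graph calls IncreaseHP.
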(event `self.ReceiveBeginPlay`
  (bind _output_get (set `self.Start` (`self.K2_GetActorLocation`)))
  (set `self.End` (+ _output_get (* (`self.GetActorUpVector`) 30.0)))
  (`TimelineComponent.SetPlayRate` (`self.RoundTrip`) 1.1)
  (bind (_direction _alpha) (`Timeline|RoundTrip`)
    (:`Update`
      (`self.K2_SetActorLocation` (`KismetMathLibrary.VLerp` (`self.Start`) (`self.End`) _alpha)))))

(event `self.StaticMeshComponent.OnComponentBeginOverlap`
  (params (OverlappedComponent :type "PrimitiveComponent Object Reference") (OtherActor :type "Actor Object Reference") (OtherComp :type "PrimitiveComponent Object Reference") (OtherBodyIndex :type Integer) (bFromSweep :type Boolean) (SweepResult :type "HitResult Structure (by ref)")))

(fn `IncreaseHP`
  (params (Player :type "/Game/Player/BP_Player Object Reference"))
  (set `/Game/Player/BP_Player.HP` (`KismetMathLibrary.FClamp` (+ (`/Game/Player/BP_Player.HP` Player) (`self.Amount`)) 0.0 (`/Game/Player/BP_Player.MaxHP` (`local.Player`))) (`local.Player`)))

(fn `UserConstructionScript`)