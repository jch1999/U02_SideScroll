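; BP_MoveCube is an input-driven actor that moves sideways and fires bullets, enabling input from player controller 0 on BeginPlay.
; The MoveRight axis event shifts it along world Y without sweep or delta-time scaling and adds a fixed yaw step each call, regardless of axis value.
; Left mouse press spawns BP_Bullet at the actor's location and rotation.
; Tick prints the current MoveRight value to screen for debugging.
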(event `self.ReceiveBeginPlay`
  (`self.EnableInput` (`GameplayStatics.GetPlayerController` 0)))

(event `InputAxis|MoveRight`
  (params (AxisValue :type "Float (single-precision)"))
  (bind (_returnvalue_roll _returnvalue_pitch _returnvalue_yaw) (`KismetMathLibrary.BreakRotator` (`self.K2_GetActorRotation`)))
  (`self.K2_SetActorLocation` (+ (* (0.0 2.0 0.0) AxisValue) (`self.K2_GetActorLocation`)))
  (`self.K2_SetActorRotation` (`KismetMathLibrary.MakeRotator` _returnvalue_roll _returnvalue_pitch (+ _returnvalue_yaw 1.0))))

(event `Key|LeftMouseButton`
  (params (Key :type "Key Structure"))
  (:`Pressed`
    (`|SpawnActorFromClass` "/Game/Blueprints/BP_Bullet.BP_Bullet_C" (`KismetMathLibrary.MakeTransform` (`self.K2_GetActorLocation`) (`self.K2_GetActorRotation`)) "Undefined" "OverrideRootScale" null null)))

(event `self.ReceiveTick`
  (params (DeltaSeconds :type "Float (single-precision)"))
  (`KismetSystemLibrary.PrintString` (`KismetStringLibrary.Conv_DoubleToString` (`self.GetInputAxisValue`)) true true (struct :`G` 0.66 :`B` 1.0 :`A` 1.0) DeltaSeconds))

(fn `UserConstructionScript`)