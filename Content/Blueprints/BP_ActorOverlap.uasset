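; BP_ActorOverlap is an actor whose point light turns on while another actor overlaps it.
; The light starts hidden at BeginPlay, shows on ActorBeginOverlap and hides again on ActorEndOverlap.
; The construction script applies the LightColor variable to the light, so the color updates in the editor.
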(event `self.ReceiveBeginPlay`
  (`SceneComponent.SetVisibility` (`self.PointLight`) false false))

(event `self.ReceiveActorBeginOverlap`
  (params (OtherActor :type "Actor Object Reference"))
  (`SceneComponent.SetVisibility` (`self.PointLight`) true false))

(event `self.ReceiveActorEndOverlap`
  (params (OtherActor :type "Actor Object Reference"))
  (`SceneComponent.SetVisibility` (`self.PointLight`) false false))

(fn `UserConstructionScript`
  (`LightComponent.SetLightColor` (`self.PointLight`) (`self.LightColor`) true))