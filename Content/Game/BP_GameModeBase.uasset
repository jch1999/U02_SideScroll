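; Game mode Blueprint that owns the stage-clear and pause screens.
; On BeginPlay it sets game input and creates both widgets hidden in the viewport.
; ShowStageClearWidget waits briefly, then reveals its widget with the mouse cursor and game-and-UI input, while ShowPauseWidget reveals the pause menu, switches to UI input and pauses the game.
; A Cheat event only prints an activation message.
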(event `self.ReceiveBeginPlay`
  (`/Game/Game/BP_FunctionLibrary.InputModeToGame`)
  (bind _returnvalue (`|CreateWidget` "/Game/UI/WB_StageClear.WB_StageClear_C"))
  (bind _output_get (set `self.StageClearWidget` _returnvalue))
  (`UserWidget.AddToViewport` _output_get 0)
  (`Widget.SetVisibility` (`self.StageClearWidget`) "Hidden")
  (bind _returnvalue_2 (`|CreateWidget` "/Game/UI/WB_Pause.WB_Pause_C"))
  (bind _output_get_2 (set `self.PauseWidget` _returnvalue_2))
  (`UserWidget.AddToViewport` _output_get_2 0)
  (`Widget.SetVisibility` (`self.PauseWidget`) "Hidden"))

(event `Cheat`
  (`KismetSystemLibrary.PrintString` "치트 활성화"))

(event `ShowStageClearWidget`
  (bind _returnvalue (`GameplayStatics.GetPlayerController` 0))
  (`KismetSystemLibrary.Delay` 3.0)
  (`Widget.SetVisibility` (`self.StageClearWidget`) "Visible")
  (set `PlayerController.bShowMouseCursor` true _returnvalue)
  (`WidgetBlueprintLibrary.SetInputMode_GameAndUIEx` _returnvalue null))

(event `ShowPauseWidget`
  (`Widget.SetVisibility` (`self.PauseWidget`) "Visible")
  (`/Game/Game/BP_FunctionLibrary.InputModeToUI`)
  (`GameplayStatics.SetGamePaused` true))

(fn `UserConstructionScript`)