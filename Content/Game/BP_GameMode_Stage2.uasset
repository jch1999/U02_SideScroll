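; Game mode for Stage 2 that watches for stage completion and offers a teleport cheat.
; BeginPlay runs the parent logic, then caches the first BP_Goal, TargetPoint and BP_Player found in the level.
; Tick polls the goal's Clear flag and, through a DoOnce, disables player input and calls StageClear a single time.
; The Cheat event moves the player character to the cached target point.
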(event `Cheat`
  (`self.K2_SetActorLocation` (`GameplayStatics.GetPlayerCharacter` 0) (`self.K2_GetActorLocation` (`self.target`)) false false))

(event `self.ReceiveBeginPlay`
  (`parent.ReceiveBeginPlay`)
  (bind _outactors (`GameplayStatics.GetAllActorsOfClass` "/Game/Blueprints/BP_Goal.BP_Goal_C"))
  (set `self.Goal` (`|GetArrayItem` _outactors))
  (bind _outactors_2 (`GameplayStatics.GetAllActorsOfClass` "/Script/Engine.TargetPoint"))
  (set `self.target` (`|GetArrayItem` _outactors_2))
  (bind _outactors_3 (`GameplayStatics.GetAllActorsOfClass` "/Game/Player/BP_Player.BP_Player_C"))
  (set `self.Player` (`|GetArrayItem` _outactors_3)))

(event `self.ReceiveTick`
  (params (DeltaSeconds :type "Float (single-precision)"))
  (if (`/Game/Blueprints/BP_Goal.bClear` (`self.Goal`))
    (`/Engine/EditorBlueprintResources/StandardMacros.DoOnce` false
      (:`Completed`
        (`self.DisableInput` (`GameplayStatics.GetPlayerCharacter` 0) (`GameplayStatics.GetPlayerController` 0))
        (`self.StageClear`)))))

(fn `UserConstructionScript`)