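; Blueprint function library with shared helpers for body-hit checks and input mode switching.
; IsBodyTagValid returns true only when the component's first tag is "Body".
; InputModeToGame and InputModeToUI toggle player 0's mouse cursor and switch between game-only and UI-only input, with the mouse left unlocked in UI mode.
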(fn `InputModeToGame`
  (bind _returnvalue (`GameplayStatics.GetPlayerController` (`local.__WorldContext`)))
  (set `PlayerController.bShowMouseCursor` false _returnvalue)
  (`WidgetBlueprintLibrary.SetInputMode_GameOnly` _returnvalue))

(fn `InputModeToUI`
  (bind _returnvalue (`GameplayStatics.GetPlayerController` (`local.__WorldContext`)))
  (set `PlayerController.bShowMouseCursor` true _returnvalue)
  (`WidgetBlueprintLibrary.SetInputMode_UIOnlyEx` _returnvalue null))

(fn `Is Body Tag Valid`
  (params (`Other Comp` :type "ActorComponent Object Reference"))
  (returns (bResult :type Boolean))
  (bind _componenttags (`ActorComponent.ComponentTags` `Other Comp`))
  (if (> (`KismetArrayLibrary.Array_Length` _componenttags) 0)
    (if (== (`|GetArrayItem` _componenttags) "Body")
      (return true)
      (else
        _)))
  (return false))